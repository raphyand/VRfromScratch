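; Main game mode of the AVR framework that supplies per-level configuration objects and pawn classes.
; It builds a level info object from the current level, then lazily constructs data, controls and UI info objects from the classes it names, falling back to defaults.
; VR, non-VR and spectator pawn getters use the same level-override pattern.
; Setting the teleport movement mode updates the controls info and notifies every teleportable actor.
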(event EventBeginPlay)

(event EventTick
  (params (DeltaSeconds :type Float%20%28single-precision%29)))

(fn ConstructionScript)

(fn SetTeleportMovementMode
  (params (TeleportMovement :type Enum_Teleport_Style%20Enum :default "NewEnumerator7"))
  (Variables|/Game/AVRFramework/Blueprints/Info/BP_Info_Controls.BP_Info_Controls_C|SetTeleportMode (Info|GetInfoControls) TeleportMovement)
  (bind _outactors (Actor|GetAllActorswithInterface "/Game/AVRFramework/Interface/Interface_Teleportable.Interface_Teleportable_C"))
  (for _array_element _outactors
    (Class|InterfaceTeleportable|ConfigureTeleporter(Message) _array_element)))

(fn GetInfoData
  (Utilities|IsValid (Variables|Info|GetInfoDataObject)
    (:Is%20Valid
      _)
    (:Is%20Not%20Valid
      (Info|UpdateInfoData)))
  (return (Variables|Info|GetInfoDataObject)))

(fn UpdateInfoData
  (bind _infolevels (Info|GetInfoLevels))
  (bind _infodata (Variables|/Game/AVRFramework/Blueprints/Info/BP_Info_Level.BP_Info_Level_C|GetInfoData _infolevels))
  (if (Utilities|IsValidClass _infodata)
    (bind _returnvalue (Game|ConstructObjectfromClass _infodata self))
    (Variables|Info|SetInfoDataObject _returnvalue)
    (else
      (bind _returnvalue_2 (Game|ConstructObjectfromClass (Variables|InfoClasses|GetDefaultInfoData) self))
      (Variables|Info|SetInfoDataObject _returnvalue_2))))

(fn GetInfoControls
  (Utilities|IsValid (Variables|Info|GetInfoControlsObject)
    (:Is%20Valid
      _)
    (:Is%20Not%20Valid
      (Info|UpdateInfoControls)))
  (return (Variables|Info|GetInfoControlsObject)))

(fn GetInfoLevels
  (Utilities|IsValid (Variables|Info|GetInfoLevelsObject)
    (:Is%20Valid
      _)
    (:Is%20Not%20Valid
      (Info|UpdateInfoLevels)))
  (return (Variables|Info|GetInfoLevelsObject)))

(fn GetInfoUI
  (Utilities|IsValid (Variables|Info|GetInfoUIObject)
    (:Is%20Valid
      _)
    (:Is%20Not%20Valid
      (Info|UpdateInfoUI)))
  (return (Variables|Info|GetInfoUIObject)))

(fn UpdateInfoControls
  (bind _infolevels (Info|GetInfoLevels))
  (bind _infocontrols (Variables|/Game/AVRFramework/Blueprints/Info/BP_Info_Level.BP_Info_Level_C|GetInfoControls _infolevels))
  (Utilities|IsValid _infolevels
    (:Is%20Valid
      (if (Utilities|IsValidClass _infocontrols)
        (bind _returnvalue (Game|ConstructObjectfromClass _infocontrols self))
        (Variables|Info|SetInfoControlsObject _returnvalue)
        (else
          (bind _returnvalue_2 (Game|ConstructObjectfromClass (Variables|InfoClasses|GetDefaultInfoControls) self :!label _label))
          (Variables|Info|SetInfoControlsObject _returnvalue_2))))
    (:Is%20Not%20Valid
      (goto _label))))

(fn UpdateInfoLevels
  (bind _returnvalue (Game|ConstructObjectfromClass (CallFunction|GetCurrentLevel self) self))
  (Variables|Info|SetInfoLevelsObject _returnvalue))

(fn UpdateInfoUI
  (bind _infolevels (Info|GetInfoLevels))
  (bind _infoui (Variables|/Game/AVRFramework/Blueprints/Info/BP_Info_Level.BP_Info_Level_C|GetInfoUI _infolevels))
  (if (Utilities|IsValidClass _infoui)
    (bind _returnvalue (Game|ConstructObjectfromClass _infoui self))
    (Variables|Info|SetInfoUIObject _returnvalue)
    (else
      (bind _returnvalue_2 (Game|ConstructObjectfromClass (Variables|InfoClasses|GetDefaultInfoUI) self))
      (Variables|Info|SetInfoUIObject _returnvalue_2))))

(fn GetVRPawnClass
  (bind _infolevels (Info|GetInfoLevels))
  (bind _pawn_vr (Variables|/Game/AVRFramework/Blueprints/Info/BP_Info_Level.BP_Info_Level_C|GetPawn_VR _infolevels))
  (Utilities|IsValid _infolevels
    (:Is%20Valid
      (if (Utilities|IsValidClass _pawn_vr)
        (return _pawn_vr)
        (else
          _)))
    (:Is%20Not%20Valid
      _))
  (return (Variables|Pawns|GetPawn_VR)))

(fn GetNonPawnClass
  (bind _infolevels (Info|GetInfoLevels))
  (bind _pawn_nonvr (Variables|/Game/AVRFramework/Blueprints/Info/BP_Info_Level.BP_Info_Level_C|GetPawn_NonVR _infolevels))
  (Utilities|IsValid _infolevels
    (:Is%20Valid
      (if (Utilities|IsValidClass _pawn_nonvr)
        (return _pawn_nonvr)
        (else
          _)))
    (:Is%20Not%20Valid
      _))
  (return (Variables|Pawns|GetPawn_NonVR)))

(fn GetSpectatorClass
  (bind _infolevels (Info|GetInfoLevels))
  (bind _pawn_spectator (Variables|/Game/AVRFramework/Blueprints/Info/BP_Info_Level.BP_Info_Level_C|GetPawn_Spectator _infolevels))
  (Utilities|IsValid _infolevels
    (:Is%20Valid
      (if (Utilities|IsValidClass _pawn_spectator)
        (return _pawn_spectator)
        (else
          _)))
    (:Is%20Not%20Valid
      _))
  (return (Variables|Pawns|GetPawn_Spectator)))